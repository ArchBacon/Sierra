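; Drivable physics vehicle that simulates four raycast wheels by applying forces to a single Chassis body.
; Each Tick traces down from the suspension points for spring-damper forces, places and spins wheel meshes, and cancels most sideways velocity for grip.
; Steering yaws the front suspension points, redirecting that grip, while throttle pushes at grounded rear points using TorqueCurve, capped at TopSpeed.
; Look input rotates the SpringArm; tire-track decals and most debug drawing are disconnected.
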(event Input|EnhancedActionEvents|EnhancedInputActionIA_Throttle
  (params (ActionValue :type Float%20%28double-precision%29) (ElapsedSeconds :type Float%20%28double-precision%29) (TriggeredSeconds :type Float%20%28double-precision%29) (InputAction :type Input%20Action%20Object%20Reference :default "/Game/Sierra/Input/IA_Throttle.IA_Throttle"))
  (CallFunction|CalculateAcceleration ActionValue))

(event Input|EnhancedActionEvents|EnhancedInputActionIA_Look
  (params (ActionValue :type Float%20%28double-precision%29) (ElapsedSeconds :type Float%20%28double-precision%29) (TriggeredSeconds :type Float%20%28double-precision%29) (InputAction :type Input%20Action%20Object%20Reference :default "/Game/Sierra/Input/IA_Look.IA_Look"))
  (Transformation|AddRelativeRotation (Variables|Default|GetSpringArm) (Math|Rotator|MakeRotator 0.0 0.0 ActionValue) false false))

(event EventTick
  (params (DeltaSeconds :type Float%20%28single-precision%29))
  (Suspension|UpdateSuspension false)
  (|SteerWheels(visually))
  (for (_array_element _array_index) (Suspension|GetSuspension)
    (Transformation|AddRelativeRotation (Utilities|Array|Get(acopy) (Wheel|GetWheels) _array_index) (Math|Rotator|MakeRotator (* (Math|Trig|RadiansToDegrees (/ (.Magnitude (Wheel|GetWheelForwardVelocity _array_element)) (Wheel|GetWheelRadius))) (Utilities|Time|GetWorldDeltaSeconds)) 0.0 0.0) false false)
    (bind _returnvalue (CallFunction|TryFindGround _array_element))
    (if _returnvalue
      (Class|PrimitiveComponent|AddForceatLocation (Variables|Default|GetChassis) (* (* (Math|Vector|NegateVector (.Direction (Wheel|GetWheelRightVelocity _array_element))) (.Magnitude (Wheel|GetWheelRightVelocity _array_element)) (select (>= _array_index 2) (Math|Float|MakeLiteralFloat 0.95) (Math|Float|MakeLiteralFloat 0.95))) (Physics|GetMass (Variables|Default|GetChassis))) (Transformation|GetWorldLocation _array_element) "None"))))

(fn ConstructionScript
  (|SetWheelstoDefaultPosition))

(fn GetWheelRadius
  (return (.SphereRadius (Math|BoxSphereBounds|BreakBoxSphereBounds (StaticMesh|GetBounds (Variables|Default|GetWheel))))))

(fn GetSuspension
  (return (Utilities|Array|MakeArray (Variables|Default|GetSuspension_FL) (Variables|Default|GetSuspension_FR) (Variables|Default|GetSuspension_RL) (Variables|Default|GetSuspension_RR))))

(fn UpdateSuspension
  (params (Debug :type Boolean))
  (for _array_element (Suspension|GetSuspension)
    (LocalVariables|SetSuspension _array_element)
    (bind (_returnvalue _outhit) (CallFunction|TryFindGround (LocalVariables|GetSuspension)))
    (if _returnvalue
      (bind _returnvalue_2 (Suspension|CalculateSuspensionForce (LocalVariables|GetSuspension) (.Distance (Collision|BreakHitResult _outhit)) (Wheel|GetWheelRadius) Debug))
      (Class|PrimitiveComponent|AddForceatLocation (Variables|Default|GetChassis) _returnvalue_2 (Transformation|GetWorldLocation (LocalVariables|GetSuspension)) "None")
      (Transformation|SetWorldLocation (Components|GetChildComponent (LocalVariables|GetSuspension) 0) (+ (Transformation|GetWorldLocation (LocalVariables|GetSuspension)) (* (Math|Vector|GetUpVector (LocalVariables|GetSuspension)) (- (.Distance (Collision|BreakHitResult _outhit)) (Wheel|GetWheelRadius)) -1.0)) false false)
      (if Debug
        (Rendering|Debug|DrawDebugArrow (Transformation|GetWorldLocation (LocalVariables|GetSuspension)) (+ (Transformation|GetWorldLocation (LocalVariables|GetSuspension)) (* (Math|Vector|GetUpVector (LocalVariables|GetSuspension)) (- (.Distance (Collision|BreakHitResult _outhit)) (Wheel|GetWheelRadius)) -1.0)) 1e+02 "(R=1.000000,G=0.000000,B=0.751215,A=1.000000)" 0.0 5.0 "Foreground"))
      (else
        (|SetWheelstoDefaultLocation)))))

(fn CalculateSuspensionForce
  (params (Suspension :type Scene%20Component%20Object%20Reference) (Distance :type Float%20%28double-precision%29) (WheelRadius :type Float%20%28double-precision%29) (Debug :type Boolean))
  (bind _returnvalue (|SuspensionForce))
  (bind _returnvalue_2 (Math|Vector|GetUpVector Suspension))
  (bind _returnvalue_3 (Transformation|GetWorldLocation Suspension))
  (bind _returnvalue_4 (* _returnvalue_2 _returnvalue))
  (bind _returnvalue_5 (Class|PrimitiveComponent|GetPhysicsLinearVelocityatPoint (Variables|Default|GetChassis) (Transformation|GetWorldLocation Suspension) "None"))
  (LocalVariables|SetSpringVelocity (Math|Vector|DotProduct _returnvalue_5 (Math|Vector|GetUpVector Suspension)))
  (if Debug
    (Rendering|Debug|DrawDebugArrow _returnvalue_3 (+ _returnvalue_3 (* _returnvalue_4 0.0005)) 1e+02 "(R=0.982251,G=1.000000,B=0.000000,A=1.000000)" 0.0 5.0 "Foreground"))
  (return _returnvalue_4))

(fn TryFindGround
  (params (Suspension :type Scene%20Component%20Object%20Reference))
  (bind _returnvalue (Transformation|GetWorldLocation Suspension))
  (bind (_outhit _returnvalue_2) (Collision|LineTraceByChannel _returnvalue (+ _returnvalue (* (Math|Vector|GetUpVector Suspension) -1.0 (+ (Variables|Suspension|GetSuspensionLength) (Wheel|GetWheelRadius)))) "TraceTypeQuery1" true 0 "None"))
  (return _returnvalue_2 _outhit))

(fn GetWheels
  (return (Utilities|Array|MakeArray (Variables|Default|GetWheel_FL) (Variables|Default|GetWheel_FR) (Variables|Default|GetWheel_RL) (Variables|Default|GetWheel_RR))))

(fn CalculateAcceleration
  (params (Alpha :type Float%20%28double-precision%29))
  (bind _chassis (Variables|Default|GetChassis))
  (bind _topspeed (Variables|Default|GetTopSpeed))
  (bind _returnvalue (Physics|GetPhysicsLinearVelocity _chassis "None"))
  (if (<= (Math|Float|Absolute(Float) (Math|Vector|DotProduct (Math|Vector|GetForwardVector _chassis) _returnvalue)) _topspeed)
    (for (_array_element _array_index) (Suspension|GetSuspension)
      (if (>= _array_index 2)
        (bind _returnvalue_2 (CallFunction|TryFindGround _array_element))
        (if _returnvalue_2
          (Class|PrimitiveComponent|AddForceatLocation (Variables|Default|GetChassis) (* (Math|Vector|GetForwardVector _array_element) (* (Math|Curves|GetFloatValue (Variables|Default|GetTorqueCurve) (Math|Float|Clamp(Float) (/ (Math|Float|Absolute(Float) (Math|Vector|DotProduct (Math|Vector|GetForwardVector _chassis) _returnvalue)) _topspeed))) Alpha) (* (Math|Float|MakeLiteralFloat 8e+02) (Physics|GetMass (Variables|Default|GetChassis)))) (Transformation|GetWorldLocation _array_element) "None"))))))

(fn GetWheelVelocity
  (params (Suspension :type Scene%20Component%20Object%20Reference))
  (bind _returnvalue (Class|PrimitiveComponent|GetPhysicsLinearVelocityatPoint (Variables|Default|GetChassis) (Transformation|GetWorldLocation Suspension) "None"))
  (return _returnvalue (Math|Vector|Normalize _returnvalue) (Math|Vector|VectorLength _returnvalue)))

(fn GetWheelForwardVelocity
  (params (Suspension :type Scene%20Component%20Object%20Reference))
  (bind _returnvalue (Math|Vector|GetForwardVector Suspension))
  (bind _returnvalue_2 (Class|PrimitiveComponent|GetPhysicsLinearVelocityatPoint (Variables|Default|GetChassis) (Transformation|GetWorldLocation Suspension) "None"))
  (return _returnvalue (Math|Vector|DotProduct _returnvalue_2 _returnvalue)))

(fn GetWheelRightVelocity
  (params (Suspension :type Scene%20Component%20Object%20Reference))
  (bind _returnvalue (Math|Vector|GetRightVector Suspension))
  (bind _returnvalue_2 (Class|PrimitiveComponent|GetPhysicsLinearVelocityatPoint (Variables|Default|GetChassis) (Transformation|GetWorldLocation Suspension) "None"))
  (return _returnvalue (Math|Vector|DotProduct _returnvalue_2 _returnvalue)))

(fn DrawWheelDebug
  (params (Suspension :type Scene%20Component%20Object%20Reference))
  (bind (_direction _magnitude) (Wheel|GetWheelRightVelocity Suspension))
  (bind (_direction_2 _magnitude_2) (Wheel|GetWheelRightVelocity Suspension))
  (bind (_direction_3 _magnitude_3) (Wheel|GetWheelRightVelocity Suspension))
  (bind _returnvalue (Transformation|GetWorldLocation Suspension))
  (Utilities|FlowControl|Sequence
    (:then_0
      (bind _output_get (LocalVariables|SetSuspensionLocation _returnvalue))
      (Rendering|Debug|DrawDebugArrow _output_get (+ _returnvalue (* (.Direction (Wheel|GetWheelVelocity Suspension)) 2e+02)) 1e+02 "(R=1.000000,G=0.243449,B=0.000000,A=1.000000)" 0.0 5.0 "Foreground") ; Velocity
    )
    (:then_1
      (Rendering|Debug|DrawDebugArrow (LocalVariables|GetSuspensionLocation) (+ (LocalVariables|GetSuspensionLocation) (* (.Direction (Wheel|GetWheelForwardVelocity Suspension)) 2e+02)) 1e+02 "(R=0.000000,G=0.000000,B=1.000000,A=1.000000)" 0.0 5.0 "Foreground") ; Rolling Direction
    )
    (:then_2
      (Rendering|Debug|DrawDebugArrow (LocalVariables|GetSuspensionLocation) (+ (LocalVariables|GetSuspensionLocation) (* _direction _magnitude)) 1e+02 "(R=1.000000,G=0.000000,B=0.000000,A=1.000000)" 0.0 5.0 "Foreground") ; Slipping Direction
    )
    (:then_3
      (Rendering|Debug|DrawDebugArrow (+ (+ (LocalVariables|GetSuspensionLocation) (* _direction_3 _magnitude_3)) (* (Math|Vector|GetForwardVector Suspension) 2e+01)) (+ (+ (+ (LocalVariables|GetSuspensionLocation) (* _direction_3 _magnitude_3)) (* (Math|Vector|GetForwardVector Suspension) 2e+01)) (* (Math|Vector|NegateVector _direction_2) _magnitude_2 (Math|Float|MakeLiteralFloat 1.0))) 1e+02 "(R=1.000000,G=0.338542,B=0.813702,A=1.000000)" 0.0 5.0 "Foreground") ; Right
    )))