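; Player vehicle Blueprint with custom raycast-wheel physics, still a work in progress with empty brake and steer handlers.
; Each tick, four suspension points trace downward, apply mass-scaled spring-damper forces to the body and reposition wheel meshes.
; CalcAccel adds torque-curve throttle force scaled by forward speed, but Tick passes it no suspension and its top-speed branch is empty.
; Look input rotates the spring arm, and debug shapes visualize forces and velocities.
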(event Input|EnhancedActionEvents|EnhancedInputActionIA_Throttle
  (params (ActionValue :type Float%20%28double-precision%29) (ElapsedSeconds :type Float%20%28double-precision%29) (TriggeredSeconds :type Float%20%28double-precision%29) (InputAction :type Input%20Action%20Object%20Reference :default "/Game/Sierra/Input/IA_Throttle.IA_Throttle")))

(event Input|EnhancedActionEvents|EnhancedInputActionIA_Brake
  (params (ActionValue :type Float%20%28double-precision%29) (ElapsedSeconds :type Float%20%28double-precision%29) (TriggeredSeconds :type Float%20%28double-precision%29) (InputAction :type Input%20Action%20Object%20Reference :default "/Game/Sierra/Input/IA_Brake.IA_Brake")))

(event Input|EnhancedActionEvents|EnhancedInputActionIA_Steer
  (params (ActionValue :type Float%20%28double-precision%29) (ElapsedSeconds :type Float%20%28double-precision%29) (TriggeredSeconds :type Float%20%28double-precision%29) (InputAction :type Input%20Action%20Object%20Reference :default "/Game/Sierra/Input/IA_Steer.IA_Steer")))

(event Input|EnhancedActionEvents|EnhancedInputActionIA_Look
  (params (ActionValue :type Float%20%28double-precision%29) (ElapsedSeconds :type Float%20%28double-precision%29) (TriggeredSeconds :type Float%20%28double-precision%29) (InputAction :type Input%20Action%20Object%20Reference :default "/Game/Sierra/Input/IA_Look.IA_Look"))
  (Transformation|AddRelativeRotation (Variables|Default|GetSpringArm) (Math|Rotator|MakeRotator 0.0 0.0 ActionValue) false false))

(event EventTick
  (params (DeltaSeconds :type Float%20%28single-precision%29))
  (bind (_keypin _valuepin) (Utilities|Map|ForEachLoop(Map) (CallFunction|GetWheelMap))
    (:then
      (Suspension|HandleWheelForces _keypin _valuepin)
      (bind _returnvalue (Class|PrimitiveComponent|GetPhysicsLinearVelocityatPoint (Variables|Default|GetBody) (Transformation|GetWorldLocation _valuepin) "None"))
      (Rendering|Debug|DrawDebugArrow (Transformation|GetWorldLocation _valuepin) (+ (Transformation|GetWorldLocation _valuepin) (* (Math|Vector|GetForwardVector _keypin) (Math|Vector|DotProduct (Math|Vector|GetForwardVector _keypin) _returnvalue))) 1e+02 "(R=1.000000,G=0.122912,B=0.000454,A=1.000000)" 0.0 5.0 "Foreground")
      (CallFunction|CalcAccel))))

(fn ConstructionScript
  (bind _valuepin (Utilities|Map|ForEachLoop(Map) (CallFunction|GetWheelMap))
    (:then
      (Transformation|AddRelativeLocation _valuepin (Math|Vector|MakeVector 0.0 0.0 (+ (* (Variables|Suspension|GetSuspensionRestDistance) -1.0) 35.0)) false false))))

(fn HandleWheelForces
  (params (Suspension :type Scene%20Component%20Object%20Reference) (Wheel :type Scene%20Component%20Object%20Reference))
  (bind _returnvalue (Transformation|GetWorldLocation Suspension))
  (bind (_outhit _returnvalue_2) (Collision|LineTraceByChannel _returnvalue (+ _returnvalue (* (Math|Vector|GetUpVector Suspension) -1.0 (Variables|Suspension|GetSuspensionRestDistance))) "TraceTypeQuery1" false 0 "None"))
  (if _returnvalue_2
    (Suspension|CalcSuspension Suspension (.Distance (Collision|BreakHitResult _outhit)))
    (Class|KismetSystemLibrary|DrawDebugCylinder (+ (.ImpactPoint (Collision|BreakHitResult _outhit)) (Math|Vector|MakeVector 0.0 0.0 (.Z (Math|Vector|BreakVector (.BoxExtent (Collision|GetComponentBounds Wheel)))))) (+ (+ (.ImpactPoint (Collision|BreakHitResult _outhit)) (Math|Vector|MakeVector 0.0 0.0 (.Z (Math|Vector|BreakVector (.BoxExtent (Collision|GetComponentBounds Wheel)))))) (Math|Vector|GetRightVector Suspension)) 35.0 12 "(R=0.000000,G=0.434783,B=1.000000,A=1.000000)" 0.0 5.0 "Foreground")
    (Transformation|SetWorldLocation Wheel (+ (.ImpactPoint (Collision|BreakHitResult _outhit)) (Math|Vector|MakeVector 0.0 0.0 (.Z (Math|Vector|BreakVector (.BoxExtent (Collision|GetComponentBounds Wheel)))))) false false)
    (else
      (Transformation|SetWorldLocation Wheel (+ (Transformation|GetWorldLocation Suspension) (* (Math|Vector|GetUpVector Suspension) -1.0 (Variables|Suspension|GetSuspensionRestDistance)) (Math|Vector|MakeVector 0.0 0.0 (.Z (Math|Vector|BreakVector (.BoxExtent (Collision|GetComponentBounds Wheel)))))) false false))))

(fn CalcSuspension
  (params (Wheel :type Scene%20Component%20Object%20Reference) (Distance :type Float%20%28double-precision%29))
  (bind _body (Variables|Default|GetBody))
  (bind _returnvalue (Transformation|GetWorldLocation Wheel))
  (bind _returnvalue_2 (Class|PrimitiveComponent|GetPhysicsLinearVelocityatPoint (Variables|Default|GetBody) (Transformation|GetWorldLocation Wheel) "None"))
  (Variables|Suspension|SetSpringVelocity (Math|Vector|DotProduct _returnvalue_2 (Math|Vector|GetUpVector Wheel)))
  (Class|PrimitiveComponent|AddForceatLocation (Variables|Default|GetBody) (* (Math|Vector|GetUpVector Wheel) (- (* (- (Variables|Suspension|GetSuspensionRestDistance) Distance) (* (Physics|GetMass _body) (Variables|Suspension|GetSpringStrength))) (* (* (Physics|GetMass _body) (Variables|Suspension|GetSuspensionDamping)) (Variables|Suspension|GetSpringVelocity)))) _returnvalue "None")
  (Rendering|Debug|DrawDebugArrow _returnvalue (+ (* (* (Math|Vector|GetUpVector Wheel) (- (* (- (Variables|Suspension|GetSuspensionRestDistance) Distance) (* (Physics|GetMass _body) (Variables|Suspension|GetSpringStrength))) (* (* (Physics|GetMass _body) (Variables|Suspension|GetSuspensionDamping)) (Variables|Suspension|GetSpringVelocity)))) 0.0005) _returnvalue) 1e+02 "(R=0.983815,G=0.000000,B=1.000000,A=1.000000)" 0.0 5.0 "Foreground"))

(fn GetWheelMap
  (return (Utilities|Map|MakeMap (Variables|Default|GetSuspension_FR) (Variables|Default|GetWheelMesh_FR) (Variables|Default|GetSuspension_FL) (Variables|Default|GetWheelMesh_FL) (Variables|Default|GetSuspension_RR) (Variables|Default|GetWheelMesh_RR) (Variables|Default|GetSuspension_RL) (Variables|Default|GetWheelMesh_RL))))

(fn CalcAccel
  (params (Suspension :type Scene%20Component%20Object%20Reference))
  (bind _body (Variables|Default|GetBody))
  (bind _returnvalue (Components|GetChildComponent Suspension 0))
  (bind _returnvalue_2 (Transformation|GetWorldLocation _returnvalue))
  (if (> (Input|EnhancedActionValues|GetIA_Throttle) 0.0)
    (bind _returnvalue_3 (Physics|GetPhysicsLinearVelocity _body "None"))
    (Development|PrintString (Utilities|String|ToString(Float) (Math|Vector|DotProduct (Math|Vector|GetForwardVector _body) _returnvalue_3)))
    (if (<= (Math|Vector|DotProduct (Math|Vector|GetForwardVector _body) _returnvalue_3) (Variables|Default|GetTopSpeed))
      _
      (else
        _))
    (Class|PrimitiveComponent|AddForceatLocation (Variables|Default|GetBody) (* (Variables|Default|GetAcceleration) (* (Math|Curves|GetFloatValue (Variables|Default|GetTorqueCurve) (Math|Float|Clamp(Float) (/ (Math|Float|Absolute(Float) (Math|Vector|DotProduct (Math|Vector|GetForwardVector _body) _returnvalue_3)) (Variables|Default|GetTopSpeed)))) (Input|EnhancedActionValues|GetIA_Throttle)) (Math|Vector|GetForwardVector Suspension)) _returnvalue_2 "None")
    (Rendering|Debug|DrawDebugArrow _returnvalue_2 (+ (* (* (Variables|Default|GetAcceleration) (* (Math|Curves|GetFloatValue (Variables|Default|GetTorqueCurve) (Math|Float|Clamp(Float) (/ (Math|Float|Absolute(Float) (Math|Vector|DotProduct (Math|Vector|GetForwardVector _body) _returnvalue_3)) (Variables|Default|GetTopSpeed)))) (Input|EnhancedActionValues|GetIA_Throttle)) (Math|Vector|GetForwardVector Suspension)) 0.01) _returnvalue_2) 1e+02 "(R=1.000000,G=0.000000,B=0.010266,A=1.000000)" 0.0 5.0 "Foreground")))