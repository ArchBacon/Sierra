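; Drivable 1987 Buick Grand National vehicle Blueprint that adds a HUD and handles steering, wheel visuals, camera look and reset.
; Tick eases front suspension yaw toward steer input, then spins grounded wheels from chassis point velocity and configured front tire diameter.
; Grounded corners with wheels apply mass-scaled force against sideways velocity for grip; the front/rear grip select is hardcoded to one value.
; Center-of-mass debug drawing is disconnected.
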(event Input|EnhancedActionEvents|EnhancedInputActionIA_Reset
  (params (ActionValue :type Boolean) (ElapsedSeconds :type Float%20%28double-precision%29) (TriggeredSeconds :type Float%20%28double-precision%29) (InputAction :type Input%20Action%20Object%20Reference :default "/Game/Sierra/Input/IA_Reset.IA_Reset"))
  (:Started
    (Transformation|SetActorLocationAndRotation (Variables|Default|GetResetLocation) "0.000000,-90.000000,0.000000" false true)))

(event Input|EnhancedActionEvents|EnhancedInputActionIA_Look
  (params (ActionValue :type Float%20%28double-precision%29) (ElapsedSeconds :type Float%20%28double-precision%29) (TriggeredSeconds :type Float%20%28double-precision%29) (InputAction :type Input%20Action%20Object%20Reference :default "/Game/Sierra/Input/IA_Look.IA_Look"))
  (Transformation|AddRelativeRotation (Variables|Default|GetSpringArm) (Math|Rotator|MakeRotator 0.0 0.0 ActionValue) false false))

(event EventBeginPlay
  (bind _returnvalue (UserInterface|CreateWidget "/Game/Sierra/UI/WPB_HUD.WPB_HUD_C" 0 self))
  (UserInterface|Viewport|AddtoViewport _returnvalue 0))

(event EventTick
  (params (DeltaSeconds :type Float%20%28single-precision%29))
  (bind _chassis (Variables|Default|GetChassis))
  (for _array_element (Class|PhysicsVehicle|GetFrontSuspension)
    (Transformation|SetRelativeRotation _array_element (Math|Rotator|MakeRotator 0.0 0.0 (Math|Interpolation|FInterpTo (.yaw (Variables|/Script/Engine.SceneComponent|GetRelativeRotation _array_element)) (+ (* (Input|EnhancedActionValues|GetIA_Steer) (Variables|Default|GetSteeringAngle)) 9e+01) (Utilities|Time|GetWorldDeltaSeconds) 4.0)) false false))
  (Variables|Default|SetSuspArray (Utilities|Array|MakeArray 0))
  (Utilities|Array|AppendArray (Variables|Default|GetSuspArray) (Class|PhysicsVehicle|GetRearSuspension))
  (Utilities|Array|AppendArray (Variables|Default|GetSuspArray) (Class|PhysicsVehicle|GetFrontSuspension))
  (for _array_element_2 (Variables|Default|GetSuspArray)
    (Utilities|IsValid _array_element_2
      (:Is%20Valid
        (if (Variables|/Script/Sierra.SuspensionComponent|GetbIsGrounded _array_element_2)
          (bind _returnvalue (Class|PrimitiveComponent|GetPhysicsLinearVelocityatPoint _chassis (Transformation|GetWorldLocation _array_element_2) "None"))
          (Utilities|IsValid (Variables|/Script/Sierra.SuspensionComponent|GetWheel _array_element_2)
            (:Is%20Valid
              (Transformation|AddRelativeRotation (Variables|/Script/Sierra.SuspensionComponent|GetWheel _array_element_2) (Math|Rotator|MakeRotator (* (Math|Trig|RadiansToDegrees (/ (Math|Vector|DotProduct _returnvalue (Math|Vector|GetForwardVector _array_element_2)) (CallFunction|GetWheelRadius))) (Utilities|Time|GetWorldDeltaSeconds)) 0.0 0.0) false false)
              (bind _returnvalue_2 (Class|PrimitiveComponent|GetPhysicsLinearVelocityatPoint _chassis (Transformation|GetWorldLocation _array_element_2) "None"))
              (Class|PrimitiveComponent|AddForceatLocation (Variables|Default|GetChassis) (* (* (Math|Vector|NegateVector (Math|Vector|GetRightVector _array_element_2)) (Math|Vector|DotProduct _returnvalue_2 (Math|Vector|GetRightVector _array_element_2)) (select false (Math|Float|MakeLiteralFloat 0.85) (Math|Float|MakeLiteralFloat 0.95))) (Physics|GetMass (Variables|Default|GetChassis))) (Transformation|GetWorldLocation _array_element_2) "None"))))))))

(fn ConstructionScript)

(fn GetWheelRadius
  (return (* (Variables|/Script/Sierra.TireConfig|GetDiameterFront (Variables|/Script/Sierra.VehicleConfig|GetTireConfig (Variables|Default|GetVehicleConfig))) 5e+01)))